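; BP_ControlPanel is an elevator control panel that builds one button per floor at BeginPlay.
; It adds tagged static mesh buttons from StartPosition in a grid, starting a new row after MaxHorizontalButtons.
; Each button carries an ElevatorButton tag plus its zero-based floor index and gets a one-based text label.
; The same loop tells the lift's CallElevatorButonRef to spawn a matching button for that index.
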(event EventBeginPlay
  ;[0.05098 0.05098 0.05098] Cache the information
  (Variables|Default|SetControl%20Panel%20Button%20OffsetCache (Variables|ControlPanelButton|GetControlPanelButtonOffset))
  (Variables|Default|SetMax%20Horizontal%20ButtonsCache (Variables|Default|GetMaxHorizontalButtons))
  (Variables|Default|SetStartTTransform (Transformation|GetRelativeTransform (Variables|Default|GetStartPosition)))
  (for _index (range 1 (Variables|Default|GetNumberOfFloors))
    (Variables|Default|SetCurrentLineValue _index)
    (if (> (Variables|Default|GetCurrentLineValue) (Variables|Default|GetMaxHorizontalButtons))
      (Variables|Default|SetNewLineValue (+ (Variables|Default|GetNewLineValue) (Variables|Default|GetControlPanelButtonDistanceVer)))
      (Variables|ControlPanelButton|SetControlPanelButtonOffset (Variables|Default|GetControl%20Panel%20Button%20OffsetCache))
      (Variables|Default|SetMaxHorizontalButtons (+ (Variables|Default|GetMaxHorizontalButtons) (Variables|Default|GetMax%20Horizontal%20ButtonsCache))))
    (bind _returnvalue (AddComponent|AddStaticMeshComponent false (Variables|Default|GetStartTTransform)))
    (bind _output_get (Variables|Default|SetBottonMeshRef _returnvalue))
    (Variables|/Script/Engine.ActorComponent|SetComponentTags _output_get (Utilities|Array|MakeArray "ElevatorButton" (Utilities|String|StringToName (Utilities|String|ToString(Integer) (- (Variables|Default|GetCurrentLineValue) 1)))))
    (Transformation|SetRelativeLocation (Variables|Default|GetBottonMeshRef) (Math|Vector|MakeVector (.x (.location (Variables|Default|GetStartTTransform))) (- (Variables|ControlPanelButton|GetControlPanelButtonOffset) (.y (.location (Variables|Default|GetStartTTransform)))) (- (.z (.location (Variables|Default|GetStartTTransform))) (Variables|Default|GetNewLineValue))) false false)
    (Variables|ControlPanelButton|SetControlPanelButtonOffset (- (Variables|ControlPanelButton|GetControlPanelButtonOffset) (Variables|Default|GetControlPanelButtonDistanceHor)))
    (Default|SpawnButton (Variables|/Game/LiftSystem/BP_Lift.BP_Lift_C|GetCallElevatorButonRef (Variables|Default|GetLiftRef)) (Utilities|String|StringToName (Utilities|String|ToString(Integer) (- (Variables|Default|GetCurrentLineValue) 1))))
    (bind _returnvalue_2 (AddComponent|AddTextRenderComponent false (Math|Transform|MakeTransform (Math|Vector|MakeVector (.x (Variables|/Script/Engine.SceneComponent|GetRelativeLocation (Variables|Default|GetBottonMeshRef))) (.y (Variables|/Script/Engine.SceneComponent|GetRelativeLocation (Variables|Default|GetBottonMeshRef))) (.z (Variables|/Script/Engine.SceneComponent|GetRelativeLocation (Variables|Default|GetBottonMeshRef)))) "0, 0, 0" "1.000000,1.000000,1.000000")))
    (Rendering|Components|TextRender|SetText _returnvalue_2 (Utilities|Text|ToText(Integer) (+ (Math|Conversions|ToInteger(Byte) (Utilities|String|ToString(Text) (Utilities|Text|ToText(Name) (Utilities|String|StringToName (Utilities|String|ToString(Integer) (- (Variables|Default|GetCurrentLineValue) 1)))))) 1)))))

(fn ConstructionScript)