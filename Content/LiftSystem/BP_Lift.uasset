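; BP_Lift is an elevator actor that spawns its controls and operates its doors.
; On BeginPlay it spawns a call button and an attached control panel at arrow components, passing each layout settings and a lift reference.
; GoToFloorEvent ignores requests while active, opens the doors for the current floor, or otherwise sets Active and closes them; no travel logic is present.
; A timeline scaled by DoorSpeed animates both doors by shrinking their X scale.
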(event Custom|GoToFloorEvent
  (params (Floor :type Integer))
  (if (not (Variables|Default|GetActive))
    (Variables|Default|SetFloorRef Floor)
    (if (== (Variables|Default|GetFloorRef) (Variables|Default|GetWhatFLoor))
      (CallFunction|OpenCLoseDoors true)
      (else
        (Variables|Default|SetActive true)
        (CallFunction|OpenCLoseDoors false)))))

(event Custom|OpenCLoseDoors
  (params (Open :type Boolean))
  (bind _door1 (Variables|Default|GetDoor1))
  (bind _relativescale3d (Variables|/Script/Engine.SceneComponent|GetRelativeScale3D _door1))
  ;[0.05098 0.05098 0.05098] CommentLift Doors
  (Components|Timeline|SetPlayRate (Variables|Default|GetOpenCloseTimeline) (/ 1.0 (Variables|Default|GetDoorSpeed)))
  (if Open
    (bind _newtrack_0 (Timeline|OpenCloseTimeline PlayFromStart)
      (:Update
        (Transformation|SetRelativeScale3D (Variables|Default|GetDoor2) (Math|Vector|MakeVector (Math|Float|Lerp 1.0 0.25 _newtrack_0) (.y _relativescale3d) (.z _relativescale3d)))))
    (else
      (Timeline|OpenCloseTimeline ReverseFromEnd))))

(event EventBeginPlay
  (bind _controlarrow (Variables|Default|GetControlArrow))
  (bind _returnvalue (Transformation|GetWorldLocation _controlarrow))
  ;[0.05098 0.05098 0.05098] Spawn button
  (bind _returnvalue_2 (Game|SpawnActorfromClass "/Game/LiftSystem/BP_Button.BP_Button_C" (Math|Transform|MakeTransform (.location (Transformation|GetWorldTransform (Variables|Default|GetButtonArrow))) "0, 0, 0" "1.000000,1.000000,1.000000") "Undefined" "MultiplyWithRoot" 0 (Variables|CallButton|GetCall%20Button%20Vert%20Offset) (Variables|CallButton|GetCall%20Button%20Hort%20Offset) (Variables|CallButton|GetCall%20Button%20Deph%20Offset) (Variables|CallButton|GetCall%20Button%20Mesh) self 0))
  (Variables|Default|SetCallElevatorButonRef _returnvalue_2)
  (bind _returnvalue_3 (Game|SpawnActorfromClass "/Game/LiftSystem/BP_ControlPanel.BP_ControlPanel_C" (Math|Transform|MakeTransform (Math|Vector|MakeVector (+ (.x _returnvalue) (Variables|ControlPanelPanel|GetControlPanelDepthOffset)) (+ (.y _returnvalue) (Variables|ControlPanelPanel|GetControlPanelHorOffset)) (+ (.z _returnvalue) (Variables|ControlPanelPanel|GetControlPanelVertOffset))) "0, 0, 0" "1.000000,1.000000,1.000000") "Undefined" "MultiplyWithRoot" 0 (Variables|LiftControlPanel|GetControl%20Panel%20Button%20Offset) (Variables|LiftControlPanel|GetMax%20Horizontal%20Buttons) (Variables|Floors|GetNumber%20Of%20Floors) (Variables|LiftControlPanel|GetControl%20Panel%20Button%20Distance%20Hor) (Variables|LiftControlPanel|GetControl%20Panel%20Button%20Distance%20Ver) self 0))
  (Transformation|AttachActorToActor _returnvalue_3 self "None" "KeepWorld" "KeepWorld" "KeepWorld" true))

(fn ConstructionScript)